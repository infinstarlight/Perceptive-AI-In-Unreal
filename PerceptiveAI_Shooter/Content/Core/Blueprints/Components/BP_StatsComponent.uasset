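; BP_StatsComponent tracks the owning actor's health and reports damage and death through event dispatchers.
; On BeginPlay it fills health to max and binds to the owner's OnTakeAnyDamage.
; Each positive hit fires OnAnyDamageTaken before subtracting from CurrentHealth, then fires OnCharDeath if IsDead finds health at or below zero.
; Health is not clamped, so further hits after death fire OnCharDeath again.
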(event Custom|CustomEvent_0
  (params (DamagedActor :type Actor%20Object%20Reference) (Damage :type Float%20%28single-precision%29) (DamageType :type Damage%20Type%20Object%20Reference) (InstigatedBy :type Controller%20Object%20Reference) (DamageCauser :type Actor%20Object%20Reference))
  (if (> Damage 0.0)
    (Default|CallOnAnyDamageTaken)
    (Variables|Health|SetCurrentHealth (- (Variables|Health|GetCurrentHealth) Damage))
    (if (CallFunction|IsDead?)
      (Default|CallOnCharDeath))))

(event EventBeginPlay
  (Variables|Health|SetCurrentHealth (Variables|Health|GetMaxHealth))
  (EventDispatchers|BindEventtoOnTakeAnyDamage (Components|GetOwner) (delegate Custom|CustomEvent_0)))

(fn IsDead?
  (return (<= (Variables|Health|GetCurrentHealth) 0.0)))