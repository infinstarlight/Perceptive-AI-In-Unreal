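; MasterWeapon is a hitscan weapon Blueprint, apparently the base for the game's guns.
; OnFireRequest calls FireRound, which line-traces on Visibility from the owner's eye viewpoint out to WeaponRange.
; A blocking hit applies point damage, plays the fire sound at the Muzzle socket and reports a damage event.
; Misses are silent, and the reported event location is the impact normal rather than the impact point.
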(event Custom|OnFireRequest
  (CallFunction|FireRound))

(event EventBeginPlay)

(event Collision|EventActorBeginOverlap
  (params (OtherActor :type Actor%20Object%20Reference)))

(event EventTick
  (params (DeltaSeconds :type Float%20%28single-precision%29)))

(fn ConstructionScript)

(fn FireRound
  (bind _returnvalue (Components|GetOwner))
  (bind _returnvalue_2 (Game|GetInstigatorController))
  (bind (_outlocation _outrotation) (Actor|GetActorEyesViewPoint _returnvalue))
  (bind _outhit (Collision|LineTraceByChannel _outlocation (+ _outlocation (* (Math|Vector|GetForwardVector _outrotation) (Variables|Default|GetWeaponRange))) "TraceTypeQuery1" false 0 "ForOneFrame"))
  (if (.bBlockingHit (Collision|BreakHitResult _outhit))
    (bind _returnvalue_3 (Game|Damage|ApplyPointDamage (.HitActor (Collision|BreakHitResult _outhit)) (Variables|Default|GetBase%20Damage) (.ImpactNormal (Collision|BreakHitResult _outhit)) _outhit _returnvalue_2 self))
    (Audio|PlaySoundatLocation "/Game/Core/FirstPerson/Audio/FirstPersonTemplateWeaponFire02.FirstPersonTemplateWeaponFire02" (Transformation|GetSocketLocation (Variables|Default|GetSkeletalMesh) "Muzzle") "0, 0, 0" 1.0 1.0 0.0 0 0 0)
    (Class|AISenseDamage|ReportDamageEvent (.HitActor (Collision|BreakHitResult _outhit)) _returnvalue_2 _returnvalue_3 (.ImpactNormal (Collision|BreakHitResult _outhit)) "0, 0, 0" "None")))