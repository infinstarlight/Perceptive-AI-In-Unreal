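; BP_NPC_MasterGuard is a guard NPC that spawns its default weapon on BeginPlay and attaches it to a hand-agnostic WeaponSocket on its mesh.
; It exposes team ID and death status, the latter read from its stats component, and forwards state changes to the AnimInstance.
; On death, it ragdolls body and weapon, expires both shortly after, and spawns a replacement of its own class at its transform just before removal.
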(event OnAnyDamageTaken(BP_StatsComponent))

(event OnCharDeath(BP_StatsComponent)
  (bind _mesh (Variables|Character|GetMesh))
  (Utilities|FlowControl|DoOnce false
    (:Completed
      (Collision|SetCollisionProfileName _mesh "Ragdoll" true :!class /Script/Engine.PrimitiveComponent)
      (Class|SkeletalMeshComponent|SetAllBodiesSimulatePhysics _mesh true)
      (Collision|SetCollisionEnabled (Variables|Collision|GetCapsuleComponent) "QueryAndPhysics")
      (Class|Log|DebugMessage "DL_Info" (Utilities|String|Append (Utilities|GetDisplayName self) " " "is Dead!") "LO_Viewport" false 5.0)
      (Actor|SetLifeSpan 3.0)
      (Actor|SetLifeSpan (Variables|Default|GetCurrentWeapon) 3.0)
      (Utilities|FlowControl|Delay 2.95)
      (Game|SpawnActorfromClass (Utilities|GetClass self) (Transformation|GetActorTransform) "Undefined" 0 0))))

(event EventBeginPlay
  (bind _self self)
  (bind _returnvalue (Game|SpawnActorfromClass (Variables|Config|GetDefaultWeapon) (CallFunction|IdentityTransform) "Undefined" _self _self))
  (bind _output_get (Variables|Default|SetCurrentWeapon _returnvalue))
  (Transformation|AttachComponentToComponent _output_get (Variables|Character|GetMesh) "WeaponSocket" "SnapToTarget" "SnapToTarget" "SnapToTarget" true))

(event Collision|EventActorBeginOverlap
  (params (OtherActor :type Actor%20Object%20Reference)))

(event EventTick
  (params (DeltaSeconds :type Float%20%28single-precision%29)))

(event EventOnStateChange
  (params (NewState :type ENPCState%20Enum :default "NewEnumerator0"))
  (Class|BPIAICommunication|OnStateChange(Message) (Components|SkeletalMesh|GetAnimInstance (Variables|Character|GetMesh)) NewState))

(fn ConstructionScript)

(fn GetTeamID
  (return (Variables|Default|GetTeamID)))

(fn IsDead?
  (return (Default|IsDead? (Variables|Default|GetBP_StatsComponent))))