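; AI controller for guard NPCs that runs the guard behavior tree and stores the NPC state in the blackboard.
; SetNewState writes the state, notifies the controlled pawn, then calls a per-state handler.
; Investigating, Searching and Alert handlers fill move location, point of interest or target keys, while Calm, Stunned and Dead are stubs.
; GetTeamID returns a fixed team and IsDead? always returns false.
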(event EventBeginPlay
  (Class|AIController|UseBlackboard "/Game/Core/AI/Blackboards/BB_Guard.BB_Guard")
  (AI|RunBehaviorTree "/Game/Core/AI/BehaviorTrees/MBT_Guard.MBT_Guard"))

(event EventTick
  (params (DeltaSeconds :type Float%20%28single-precision%29)))

(fn ConstructionScript)

(fn GetNPCState
  (return (Utilities|Enum|ByteToEnumENPCState (Class|BlackboardComponent|GetValueasEnum (Variables|Default|GetBlackboard) (Variables|Keys|GetCharStateKey)))))

(fn SetNewState
  (params (NewState :type ENPCState%20Enum :default "NewEnumerator0"))
  (bind _returnvalue (Utilities|Enum|LiteralenumENPCState NewState))
  (AI|Components|Blackboard|SetValueasEnum (Variables|Default|GetBlackboard) (Variables|Keys|GetCharStateKey) _returnvalue)
  (Class|BPIAICommunication|OnStateChange(Message) (Pawn|GetControlledPawn) _returnvalue)
  (switch Utilities|FlowControl|Switch|SwitchonENPCState _returnvalue
    (:NewEnumerator0
      (CallFunction|OnSetCalmState))
    (:NewEnumerator1
      (CallFunction|OnSetInvestigateState))
    (:NewEnumerator2
      (CallFunction|OnSetSearchState))
    (:NewEnumerator3
      (CallFunction|OnSetAlertState))
    (:NewEnumerator4
      (CallFunction|OnSetStunnedState))
    (:NewEnumerator5
      (CallFunction|OnSetDeadState))))

(fn OnSetCalmState
  (if (Utilities|Enum|Equal(Enum) (States|GetNPCState) "NewEnumerator0")
    _))

(fn OnSetInvestigateState
  (if (Utilities|Enum|Equal(Enum) (States|GetNPCState) "NewEnumerator1")
    (AI|Components|Blackboard|SetValueasVector (Variables|Default|GetBlackboard) (Variables|Keys|GetNextLocKey) (Variables|Default|GetNewMoveToLocation))
    (AI|Components|Blackboard|SetValueasVector (Variables|Default|GetBlackboard) (Variables|Keys|GetPointOfInterestKey) (Variables|Default|GetNewPointOfInterest))))

(fn OnSetSearchState
  (if (Utilities|Enum|Equal(Enum) (States|GetNPCState) "NewEnumerator2")
    (AI|Components|Blackboard|SetValueasVector (Variables|Default|GetBlackboard) (Variables|Keys|GetNextLocKey) (Variables|Default|GetLastKnownLocation))))

(fn OnSetAlertState
  (if (Utilities|Enum|Equal(Enum) (States|GetNPCState) "NewEnumerator3")
    (AI|Components|Blackboard|SetValueasObject (Variables|Default|GetBlackboard) (Variables|Keys|GetCurrentTargetKey) (Variables|Default|GetDetectedActor))))

(fn OnSetStunnedState
  (if (Utilities|Enum|Equal(Enum) (States|GetNPCState) "NewEnumerator4")
    _))

(fn OnSetDeadState
  (if (Utilities|Enum|Equal(Enum) (States|GetNPCState) "NewEnumerator4")
    _))

(fn GetTeamID
  (return "NewEnumerator0"))

(fn IsDead?
  (return false))